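; Player-controlled car Blueprint with an orbit-style aim camera and simple digital driving controls.
; On BeginPlay it registers CarBody through SetBodyReference.
; Aim axes rotate AzimuthGimbal in yaw and SpringArm in pitch, scaled by frame time, keeping the two rotations separate.
; Forward, Left and Right actions set throttle and turn on CarBody and reset them on release, with no reverse or brake input.
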(event `self.ReceiveBeginPlay`
  (`self.SetBodyReference` (`self.CarBody`)))

(event `InputAxis|Aim Azimuth`
  (params (AxisValue :type "Float (single-precision)"))
  (`SceneComponent.K2_AddLocalRotation` (`self.Azimuth Gimbal`) (`KismetMathLibrary.MakeRotator` 0.0 0.0 (* AxisValue (`GameplayStatics.GetWorldDeltaSeconds`) 100.0)) false false))

(event `InputAxis|Aim Elevation`
  (params (AxisValue :type "Float (single-precision)"))
  (`SceneComponent.K2_AddLocalRotation` (`self.SpringArm`) (`KismetMathLibrary.MakeRotator` 0.0 (* AxisValue (`GameplayStatics.GetWorldDeltaSeconds`) 100.0)) false false))

(event `InputAction|Forward`
  (params (Key :type "Key Structure"))
  (bind _carbody (`self.CarBody`))
  (:`Pressed`
    (`CarBody.SetThrottle` _carbody 1.0))
  (:`Released`
    (`CarBody.SetThrottle` _carbody 0.0)))

(event `InputAction|Left`
  (params (Key :type "Key Structure"))
  (bind _carbody (`self.CarBody`))
  (:`Pressed`
    (`CarBody.SetTurn` _carbody -1.0))
  (:`Released`
    (`CarBody.SetTurn` _carbody 0.0 :!label _label)))

(event `InputAction|Right`
  (params (Key :type "Key Structure"))
  (:`Pressed`
    (`CarBody.SetTurn` (`self.CarBody`) 1.0))
  (:`Released`
    (goto _label)))

(fn `UserConstructionScript`)